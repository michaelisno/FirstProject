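; Exploding barrel actor that detonates on a timer after BeginPlay, or shortly after it takes radial damage.
; Explode runs once behind a flag, applying full radial damage, firing a RadialForce impulse, and spawning explosion particles and sound.
; It removes the barrel component at once and destroys the actor after a brief delay.
; The delayed reaction to radial damage lets nearby barrels set each other off in staggered chains.
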(event `self.ReceiveBeginPlay`
  (`KismetSystemLibrary.Delay` (`self.TimeToExplode`))
  (`self.Explode`))

(event `Explode`
  (bind _returnvalue (`self.K2_GetActorLocation`))
  (if (not (`self.HasExploded`))
    (set `self.HasExploded` true)
    (`GameplayStatics.ApplyRadialDamage` :`BaseDamage` 100.0 :`Origin` _returnvalue :`DamageRadius` 1000.0 :`DamageTypeClass` "/Engine/EngineDamageTypes/DmgTypeBP_Environmental.DmgTypeBP_Environmental_C" :`DamageCauser` null :`InstigatedByController` null :`bDoFullDamage` true)
    (`RadialForceComponent.FireImpulse` (`self.RadialForce`))
    (`GameplayStatics.SpawnEmitterAtLocation` "/Game/StarterContent/Particles/P_Explosion.P_Explosion" _returnvalue (struct) (2.25 2.25 2.25))
    (`GameplayStatics.SpawnSoundAtLocation` (`self.ExplosionSoundWave`) _returnvalue (struct) 1.0 1.0 0.0 null null)
    (`ActorComponent.K2_DestroyComponent` (`self.Barrel`))
    (`KismetSystemLibrary.Delay` 1.0)
    (`self.K2_DestroyActor`)))

(event `self.ReceiveRadialDamage`
  (params (DamageReceived :type "Float (single-precision)") (DamageType :type "DamageType Object Reference") (Origin :type "Vector Structure") (HitInfo :type "HitResult Structure (by ref)") (InstigatedBy :type "Controller Object Reference") (DamageCauser :type "Actor Object Reference"))
  (`KismetSystemLibrary.Delay` 0.2)
  (`self.Explode`))

(fn `UserConstructionScript`)