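; BP_Platform is a moving platform that shuttles its Cube back and forth between its starting position and EndOffset.
; On BeginPlay it stores the Cube's world location, then MoveTimeline lerps between the two world points without sweep.
; A FlipFlop on the timeline's Finished output alternates reverse and forward playback, looping the motion endlessly.
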(event `self.ReceiveBeginPlay`
  (set `self.StartOffset` (`SceneComponent.K2_GetComponentLocation` (`self.Cube`)))
  (bind (_direction _alpha) (`Timeline|MoveTimeline` :!via `PlayFromStart` :!label _label)
    (:`Update`
      (`SceneComponent.K2_SetWorldLocation` (`self.Cube`) (`KismetMathLibrary.VLerp` (`self.StartOffset`) (`self.EndOffset`) _alpha) false false))
    (:`Finished`
      (`/Engine/EditorBlueprintResources/StandardMacros.FlipFlop`
        (:`A`
          (`self.ReverseMovement`))
        (:`B`
          (goto _label))))))

(event `ReverseMovement`
  (goto _label :!via `Reverse`))

(fn `UserConstructionScript`)