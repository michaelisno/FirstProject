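; BP_ChangingSphere is an actor whose sphere component changes size and color in response to player input.
; On BeginPlay it enables input from player controller 0 and turns on that controller's click events.
; Holding L doubles the sphere's world scale, and releasing it restores normal size.
; Clicking the sphere applies a red material, and releasing the click restores the basic shape material.
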(event `self.ReceiveBeginPlay`
  (bind _returnvalue (`GameplayStatics.GetPlayerController` 0))
  (`self.EnableInput` _returnvalue)
  (set `PlayerController.bEnableClickEvents` true _returnvalue))

(event `Key|L`
  (params (Key :type "Key Structure"))
  (bind _sphere (`self.Sphere`))
  (:`Pressed`
    (`SceneComponent.SetWorldScale3D` _sphere (2.0 2.0 2.0)))
  (:`Released`
    (`SceneComponent.SetWorldScale3D` _sphere (1.0 1.0 1.0))))

(event `self.Sphere.OnClicked`
  (params (TouchedComponent :type "PrimitiveComponent Object Reference") (ButtonPressed :type "Key Structure"))
  (`PrimitiveComponent.SetMaterial` (`self.Sphere`) 0 "/Game/Materials/RED.RED"))

(event `self.Sphere.OnReleased`
  (params (TouchedComponent :type "PrimitiveComponent Object Reference") (ButtonReleased :type "Key Structure"))
  (`PrimitiveComponent.SetMaterial` (`self.Sphere`) 0 "/Engine/BasicShapes/BasicShapeMaterial.BasicShapeMaterial"))

(fn `UserConstructionScript`)